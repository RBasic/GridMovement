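; BP_Grid is an actor that builds a two-dimensional grid of BP_Cell actors.
; InitGrid destroys the previously stored cells and clears the array, then spawns new cells in nested X and Y loops and stores each one.
; Cell positions come from loop index times per-axis spacing, with no offset from the grid actor's location.
; The event graph and construction script are empty, so InitGrid is not called within this Blueprint.
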(event EventBeginPlay)

(event Collision|EventActorBeginOverlap
  (params (OtherActor :type Actor%20Object%20Reference)))

(event EventTick
  (params (DeltaSeconds :type Float%20%28single-precision%29)))

(fn ConstructionScript)

(fn InitGrid
  (bind _newvar (Variables|Default|GetNewVar))
  (for _array_element _newvar
    (Actor|DestroyActor _array_element))
  (Utilities|Array|Clear _newvar)
  (for _index (range 0 (Variables|Default|GetSizeX))
    (for _index_2 (range 0 (Variables|Default|GetSizeY))
      (bind _returnvalue (Game|SpawnActorfromClass "/Game/Core/BP_Cell.BP_Cell_C" (Math|Transform|MakeTransform (Math|Vector|MakeVector (* _index (Variables|Default|GetSpaceX)) (* _index_2 (Variables|Default|GetSpaceY)) 0.0) "0, 0, 0" "1.000000,1.000000,1.000000") "Undefined" 0 0))
      (Utilities|Array|Add (Variables|Default|GetNewVar) _returnvalue))))