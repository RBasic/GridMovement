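; BP_Cell is a graph node actor, apparently for Dijkstra pathfinding, with a dynamic sphere material and a text label showing its name.
; RefreshNeighbors compares every pair of cells, updating parallel neighbor and distance arrays using the DistMin threshold.
; It then calls ShowAllNeighbors, which draws temporary debug lines from a separate Neighbors map rather than those arrays.
; The Dijkstra call in the construction script is disconnected.
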(event EventBeginPlay)

(event Collision|EventActorBeginOverlap
  (params (OtherActor :type Actor%20Object%20Reference)))

(event EventTick
  (params (DeltaSeconds :type Float%20%28single-precision%29)))

(fn ConstructionScript
  (Utilities|FlowControl|Sequence
    (:then_0
      (bind _returnvalue (Rendering|Material|CreateDynamicMaterialInstance (Variables|Default|GetSphere) 0 "/Engine/BasicShapes/BasicShapeMaterial.BasicShapeMaterial" "None" :!class /Script/Engine.PrimitiveComponent))
      (Variables|Default|SetMat _returnvalue))
    (:then_2
      (Rendering|Components|TextRender|SetText (Variables|Default|GetTextRender) (Utilities|Text|ToText(String) (Utilities|GetDisplayName self))))))

(fn RefreshNeighbors
  (bind _outactors (Actor|GetAllActorsOfClass "BP_Cell_C"))
  (bind _output_get (LocalVariables|SetCells _outactors))
  (for _array_element _output_get
    (LocalVariables|SetCellA _array_element)
    (for _array_element_2 (LocalVariables|GetCells)
      (LocalVariables|SetCellB _array_element_2)
      (if (!= (LocalVariables|GetCellA) (LocalVariables|GetCellB))
        (if (<= (Math|Vector|Distance(Vector) (Transformation|GetActorLocation (LocalVariables|GetCellA)) (Transformation|GetActorLocation (LocalVariables|GetCellB))) (Variables|Default|GetDistMin))
          (Utilities|Array|Add (Variables|BP_Cell_C|GetNeighborsCell (LocalVariables|GetCellA)) (LocalVariables|GetCellB))
          (Utilities|Array|Add (Variables|BP_Cell_C|GetDistNeighbors (LocalVariables|GetCellA)) (Math|Vector|Distance(Vector) (Transformation|GetActorLocation (LocalVariables|GetCellA)) (Transformation|GetActorLocation (LocalVariables|GetCellB))))
          (else
            (Utilities|Array|RemoveIndex (Variables|BP_Cell_C|GetDistNeighbors (LocalVariables|GetCellA)) (Utilities|Array|FindItem (Variables|BP_Cell_C|GetNeighborsCell (LocalVariables|GetCellA)) (LocalVariables|GetCellB)))
            (Utilities|Array|RemoveIndex (Variables|BP_Cell_C|GetNeighborsCell (LocalVariables|GetCellA)) (Utilities|Array|FindItem (Variables|BP_Cell_C|GetNeighborsCell (LocalVariables|GetCellA)) (LocalVariables|GetCellB))))))))
  (CallFunction|ShowAllNeighbors))

(fn ShowAllNeighbors
  (Rendering|Debug|FlushPersistentDebugLines)
  (bind _outactors (Actor|GetAllActorsOfClass "BP_Cell_C"))
  (for _array_element _outactors
    (bind _keys (Utilities|Map|Keys (Variables|BP_Cell_C|GetNeighbors _array_element)))
    (for _array_element_2 _keys
      (Rendering|Debug|DrawDebugLine (Transformation|GetActorLocation _array_element_2) (Transformation|GetActorLocation _array_element) "(R=0.765625,G=0.034789,B=0.000000,A=1.000000)" 2e+01 5.0))))